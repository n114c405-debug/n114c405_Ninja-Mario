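; Player character Blueprint for a 2D side-view game, driven by Enhanced Input through IMC_Player01, added on BeginPlay.
; Move input, gated by CanMove, moves along world X, sets the Run flipbook and rotates PaperSprite to face the travel direction.
; Jump input drives jumping with a Jump flipbook, and landing restores Idle.
; The falling check does nothing, and move release restores Idle only when the stored SetFlipbook result is false.
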(event `self.ReceiveBeginPlay`
  (`EnhancedInputSubsystemInterface.AddMappingContext` (pcsubsystem `EnhancedInputLocalPlayerSubsystem` (`GameplayStatics.GetPlayerController` 0)) "/Game/C03_01/input/IMC_Player01.IMC_Player01" 0 (struct)))

(event `EnhancedInput|/Game/C03_01/input/IA_Move01`
  (params (ActionValue :type "Vector2D Structure") (ElapsedSeconds :type "Float (double-precision)") (TriggeredSeconds :type "Float (double-precision)") (InputAction :type "InputAction Object Reference" :default "/Game/C03_01/input/IA_Move01.IA_Move01"))
  (bind _x (`KismetMathLibrary.BreakVector2D` ActionValue))
  (bind _papersprite (`self.PaperSprite`))
  (:`Triggered`
    (if (`self.CanMove`)
      (if (> _x 0.0)
        (set `self.isFacingRight` true)
        (else
          (set `self.isFacingRight` false)))
      (`self.AddMovementInput` (1.0 0.0 0.0) _x)
      (if (`NavMovementComponent.IsFalling` (`self.CharacterMovement`))
        _
        (else
          _))
      (bind _returnvalue (`PaperFlipbookComponent.SetFlipbook` (`self.Idle`) "/Game/C03_01/SpriteSet02/Run/Run.Run"))
      (if (`self.isFacingRight`)
        (`SceneComponent.K2_SetRelativeRotation` :`self` _papersprite)
        (else
          (`SceneComponent.K2_SetRelativeRotation` _papersprite (struct :`Yaw` 180.0) false false)))
      (else
        (`KismetSystemLibrary.PrintString` "MoveLocked"))))
  (:`Completed`
    (if (not _returnvalue)
      (`PaperFlipbookComponent.SetFlipbook` (`self.Idle`) "/Game/C03_01/SpriteSet02/ldle/Idle.Idle"))))

(event `EnhancedInput|/Game/C03_01/input/IA_Jump01`
  (params (ActionValue :type Boolean) (ElapsedSeconds :type "Float (double-precision)") (TriggeredSeconds :type "Float (double-precision)") (InputAction :type "InputAction Object Reference" :default "/Game/C03_01/input/IA_Jump01.IA_Jump01"))
  (:`Started`
    (`PaperFlipbookComponent.SetFlipbook` (`self.Idle`) "/Game/C03_01/SpriteSet02/Jump/Jump.Jump")
    (`self.Jump`))
  (:`Completed`
    (`PaperFlipbookComponent.SetFlipbook` (`self.Idle`) "/Game/C03_01/SpriteSet02/Jump/Jump.Jump")
    (`self.StopJumping`)))

(event `self.OnLanded`
  (params (Hit :type "HitResult Structure (by ref)"))
  (`PaperFlipbookComponent.SetFlipbook` (`self.Idle`) "/Game/C03_01/SpriteSet02/ldle/Idle.Idle"))

(fn `UserConstructionScript`)